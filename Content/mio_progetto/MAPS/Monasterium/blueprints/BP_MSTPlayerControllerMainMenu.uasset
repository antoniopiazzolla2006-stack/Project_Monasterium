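; Player controller for the Monasterium main menu that creates and shows the menu widget when play begins.
; BeginPlay adds WBP_MST_Main_menu to the viewport, switches input to UI only and shows the mouse cursor.
; It plays the widget's FadeOutBorder animation, waits through a delay, then plays FadeInMenu and makes an overlay visible.
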(event `self.ReceiveBeginPlay`
  (bind _wbp_main_menu (`self.WBP_main_menu`))
  (bind _wbp_main_menu_2 (`self.WBP_main_menu`))
  (bind _returnvalue (`|CreateWidget` "/Game/mio_progetto/MAPS/Monasterium/UI/WBP_MST_Main_menu.WBP_MST_Main_menu_C"))
  (bind _output_get (set `self.WBP_main_menu` _returnvalue))
  (`UserWidget.AddToViewport` _output_get 0)
  (`WidgetBlueprintLibrary.SetInputMode_UIOnlyEx` self null)
  (set `self.bShowMouseCursor` true)
  (`UserWidget.PlayAnimation` _wbp_main_menu (`/Game/mio_progetto/MAPS/Monasterium/UI/WBP_MST_Main_menu.Fade_out_border` _wbp_main_menu) 0.0 1 "Forward" 1.0 false)
  (`KismetSystemLibrary.Delay` 5.0)
  (`UserWidget.PlayAnimation` _wbp_main_menu_2 (`/Game/mio_progetto/MAPS/Monasterium/UI/WBP_MST_Main_menu.Fade_in_menu` _wbp_main_menu_2) 0.0 1 "Forward" 1.0 false)
  (`Widget.SetVisibility` (`/Game/mio_progetto/MAPS/Monasterium/UI/WBP_MST_Main_menu.Overlay_56` _wbp_main_menu_2) "Visible"))

(fn `UserConstructionScript`)