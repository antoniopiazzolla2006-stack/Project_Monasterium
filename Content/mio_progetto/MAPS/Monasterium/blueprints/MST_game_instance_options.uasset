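; Game instance for the Monasterium options, holding the master volume setting and persisting it between sessions.
; On Init it loads the options save game from the default slot, or creates one in memory if none exists, and caches the reference.
; SetVolume and SaveSettings write the value through to that save object and slot, while ResetSettings only restores the in-memory default without saving.
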(event `self.ReceiveInit`
  (`self.LoadOrCreateSaveGame`))

(fn `getVolume`
  (returns (MasterVolume :type "Float (double-precision)"))
  (return (`self.MasterVolume`)))

(fn `LoadOrCreateSaveGame`
  (bind _returnvalue (`GameplayStatics.DoesSaveGameExist` "Default"))
  (if _returnvalue
    (bind _returnvalue_2 (`GameplayStatics.LoadGameFromSlot` "Default"))
    (bind _asbp_save_game_options_mst (cast `/Game/mio_progetto/MAPS/Monasterium/blueprints/BP_save_game_Options_MST` _returnvalue_2)
      (:`then`
        (bind _output_get (set `self.As BP Save Game Options MST` _asbp_save_game_options_mst))
        (`self.SetLoadedSettingValues` _output_get))
      (:`CastFailed`
        (`KismetSystemLibrary.PrintString` "fallito")))
    (else
      (bind _returnvalue_3 (`GameplayStatics.CreateSaveGameObject` "/Game/mio_progetto/MAPS/Monasterium/blueprints/BP_save_game_Options_MST.BP_save_game_Options_MST_C"))
      (set `self.As BP Save Game Options MST` _returnvalue_3))))

(fn `ResetSettings`
  (returns (MasterVolume :type "Float (double-precision)"))
  (bind _output_get (set `self.MasterVolume` 1.0))
  (return _output_get))

(fn `SaveSettings`
  (params (MasterVolume :type "Float (double-precision)"))
  (bind _as_bp_save_game_options_mst (`self.As BP Save Game Options MST`))
  (`|ExecutionSequence`
    (:`then_0`
      (set `self.MasterVolume` MasterVolume))
    (:`then_1`
      (`/Game/mio_progetto/MAPS/Monasterium/blueprints/BP_save_game_Options_MST.SetVolume` _as_bp_save_game_options_mst MasterVolume))
    (:`then_2`
      (`GameplayStatics.SaveGameToSlot` _as_bp_save_game_options_mst "Default"))))

(fn `SetLoadedSettingValues`
  (params (Save_game_ref :type "/Game/mio_progetto/MAPS/Monasterium/blueprints/BP_save_game_Options_MST Object Reference"))
  (bind _master_volume (`/Game/mio_progetto/MAPS/Monasterium/blueprints/BP_save_game_Options_MST.GetVolume` Save_game_ref))
  (set `self.MasterVolume` _master_volume))

(fn `SetVolume`
  (params (MasterVolume :type "Float (double-precision)"))
  (set `self.MasterVolume` MasterVolume)
  (`self.UpdateSettings`))

(fn `UpdateSettings`
  (bind _as_bp_save_game_options_mst (`self.As BP Save Game Options MST`))
  (`|ExecutionSequence`
    (:`then_0`
      (`/Game/mio_progetto/MAPS/Monasterium/blueprints/BP_save_game_Options_MST.SetVolume` _as_bp_save_game_options_mst (`self.MasterVolume`)))
    (:`then_1`
      (bind _returnvalue (`GameplayStatics.SaveGameToSlot` _as_bp_save_game_options_mst "Default"))
      (if _returnvalue
        (`KismetSystemLibrary.PrintString` "salvato")
        (else
          (`KismetSystemLibrary.PrintString` "non salvato"))))))